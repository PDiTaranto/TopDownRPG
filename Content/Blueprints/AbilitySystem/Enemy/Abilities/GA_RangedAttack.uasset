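; Enemy ranged attack gameplay ability that fires a projectile at the avatar's combat target.
; On activation it turns the avatar toward the target, plays a random tagged attack montage and waits for that tag's gameplay event.
; On the event it re-reads the target's location for SpawnProjectile; the combat socket lookup result is unused.
; The graph never calls EndAbility.
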(event `self.K2_ActivateAbility`
  (bind _returnvalue (message `EnemyInterface.GetCombatTarget` (`self.GetAvatarActorFromActorInfo`)))
  (message `CombatInterface.UpdateFacingTarget` (`self.GetAvatarActorFromActorInfo`) (`Actor.K2_GetActorLocation` _returnvalue))
  (bind _returnvalue_2 (message `CombatInterface.GetAttackMontages` (`self.GetAvatarActorFromActorInfo`)))
  (bind (_item _returnvalue_3) (`AuraAbilitySystemLibrary.RandomArrayElement` _returnvalue_2))
  (if _returnvalue_3
    (bind _output_get (set `self.TaggedMontage` _item))
    (bind (_montage _tag) (break `TaggedMontage` _output_get))
    (`AbilityTask_PlayMontageAndWait.CreatePlayMontageAndWaitProxy` "None" _montage 1.0 "None" false
      (:`then`
        (`AbilityTask_WaitGameplayEvent.WaitGameplayEvent` _tag null
          (:`EventReceived`
            (message `CombatInterface.GetCombatSocketLocation` (`self.GetAvatarActorFromActorInfo`) _tag)
            (bind _returnvalue_4 (message `EnemyInterface.GetCombatTarget` (`self.GetAvatarActorFromActorInfo`)))
            (`self.SpawnProjectile` (`Actor.K2_GetActorLocation` _returnvalue_4))))))))